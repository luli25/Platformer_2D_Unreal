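; Player character for a side-scrolling action platformer, with jump, slide, wall slide and jump, and charged shooting.
; Enhanced Input drives movement and energy-costed projectiles, with slides using async root motion and Tick line traces detecting walls.
; Damage cancels slides and charging, updates the HUD and applies knockback, stun and flickering invincibility.
; Defeat detaches the camera, fades out, respawns through GM_Action and destroys the actor.
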(event `self.ReceiveBeginPlay`
  (`parent.ReceiveBeginPlay`)
  (`|ExecutionSequence`
    (:`then_0`
      (bind _asgm_action (cast `/Game/Blueprints/GM_Action` (`GameplayStatics.GetGameMode`)))
      (set `self.GameMode` _asgm_action)
      (bind _asplayer_controller (cast `PlayerController` (`self.GetController`)))
      (`EnhancedInputSubsystemInterface.AddMappingContext` (pcsubsystem `EnhancedInputLocalPlayerSubsystem` _asplayer_controller) "/Game/Assets/Input/IMC_Action.IMC_Action" 0 (struct)))
    (:`then_1`
      (set `self.BaseLateralFriction` (`CharacterMovementComponent.FallingLateralFriction` (`self.CharacterMovement`)))
      (`/Game/Widgets/WBP_HealthComponent.UpdateHealth` (`/Game/Widgets/WBP_HUD.WBP_HealthComponent` (`/Game/Blueprints/GM_Action.HUD_Ref` (`self.GameMode`))) (`/Game/Blueprints/Components/BPC_Vitality.CurrentHealth` (`self.BPC_Vitality`))))
    (:`then_2`
      (add `self.Defeated` (delegate `OnDefeated`)))))

(event `OnDefeated`
  (`PrimitiveComponent.SetCollisionEnabled` (`self.CapsuleComponent`) "NoCollision")
  (`SceneComponent.K2_DetachFromComponent` (`self.SpringArm`) "KeepWorld" "KeepWorld" "KeepWorld" true)
  (`PlayerCameraManager.StartCameraFade` :`self` (`GameplayStatics.GetPlayerCameraManager` 0) :`ToAlpha` 1.0 :`Duration` (`self.RespawnDelay`) :`bHoldWhenFinished` true)
  (`KismetSystemLibrary.Delay` (`self.RespawnDelay`))
  (`/Game/Blueprints/GM_Action.RespawnPlayer` (`self.GameMode`))
  (`PlayerCameraManager.StartCameraFade` :`self` (`GameplayStatics.GetPlayerCameraManager` 0) :`FromAlpha` 1.0 :`Duration` (`self.RespawnDelay`) :`bHoldWhenFinished` true)
  (`self.K2_DestroyActor`))

(event `self.ReceiveTick`
  (params (DeltaSeconds :type "Float (single-precision)"))
  (`parent.ReceiveTick` DeltaSeconds)
  (`self.TryWallSlide`))

(event `EnhancedInput|/Game/Assets/Input/Actions/IA_Jump`
  (params (ActionValue :type Boolean) (ElapsedSeconds :type "Float (double-precision)") (TriggeredSeconds :type "Float (double-precision)") (InputAction :type "InputAction Object Reference" :default "/Game/Assets/Input/Actions/IA_Jump.IA_Jump"))
  (bind _returnvalue_x (`KismetMathLibrary.BreakVector` (`KismetMathLibrary.GetForwardVector` (struct))))
  (:`Started`
    (if (not (`self.IsStunned`))
      (if (`self.IsWallSliding`)
        (set `CharacterMovementComponent.FallingLateralFriction` 0.0 (`self.CharacterMovement`))
        (`self.LaunchCharacter` (`KismetMathLibrary.MakeVector` (* _returnvalue_x -1.0 (`self.HorizontalJumpPower`)) 0.0 (`self.VerticalWallJumpPower`)) true true)
        (`GameplayStatics.PlaySound2D` "/Game/Assets/Sounds/Jump_Player_Cue.Jump_Player_Cue" 1.0 1.0 0.0 null null)
        (`KismetSystemLibrary.RetriggerableDelay` (`self.WallJumpLock`))
        (set `CharacterMovementComponent.FallingLateralFriction` (`self.BaseLateralFriction`) (`self.CharacterMovement`))
        (else
          (`self.Jump`)
          (`GameplayStatics.PlaySound2D` "/Game/Assets/Sounds/Jump_Player_Cue.Jump_Player_Cue" 1.0 1.0 0.0 null null)
          (`self.CancelSlide`)))))
  (:`Canceled`
    (`self.StopJumping` :!label _label))
  (:`Completed`
    (goto _label)))

(event `EnhancedInput|/Game/Assets/Input/Actions/IA_Move`
  (params (ActionValue :type "Float (double-precision)") (ElapsedSeconds :type "Float (double-precision)") (TriggeredSeconds :type "Float (double-precision)") (InputAction :type "InputAction Object Reference" :default "/Game/Assets/Input/Actions/IA_Move.IA_Move"))
  (:`Triggered`
    (if (not (`self.IsStunned`))
      (`self.AddMovementInput` (1.0 0.0 0.0) ActionValue)
      (`self.FlipPlayer` ActionValue))))

(event `EnhancedInput|/Game/Assets/Input/Actions/IA_Shoot`
  (params (ActionValue :type Boolean) (ElapsedSeconds :type "Float (double-precision)") (TriggeredSeconds :type "Float (double-precision)") (InputAction :type "InputAction Object Reference" :default "/Game/Assets/Input/Actions/IA_Shoot.IA_Shoot"))
  (:`Started`
    (if (and (not (`self.IsStunned`)) (not (`self.IsSliding`)))
      (set `self.WasHitDuringCharge` false)
      (`self.SpawnProjectile` "/Game/Blueprints/Projectiles/Player/BP_PlayerProjectile_Regular.BP_PlayerProjectile_Regular_C")))
  (:`Ongoing`
    (`self.HandleChargeFlash` ElapsedSeconds))
  (:`Completed`
    (if (and (not (`self.IsStunned`)) (not (`self.IsSliding`)))
      (`self.TryChargeShot` ElapsedSeconds)
      (`ActorComponent.Deactivate` (`self.ChargeShot`)))))

(event `self.CapsuleComponent.OnComponentBeginOverlap`
  (params (OverlappedComponent :type "PrimitiveComponent Object Reference") (OtherActor :type "Actor Object Reference") (OtherComp :type "PrimitiveComponent Object Reference") (OtherBodyIndex :type Integer) (bFromSweep :type Boolean) (SweepResult :type "HitResult Structure (by ref)"))
  (bind _asbp_enemy_base (cast `/Game/Blueprints/Characters/Enemies/BP_Enemy_BASE` OtherActor))
  (if (== (`Character.CapsuleComponent` _asbp_enemy_base) OtherComp)
    (`GameplayStatics.ApplyDamage` self (`self.EnemyDamage`) null _asbp_enemy_base)))

(event `CancelSlide`
  (`/Engine/EditorBlueprintResources/StandardMacros.IsValid` (stale `EnhancedInput|/Game/Assets/Input/Actions/IA_Slide` _asynctaskproxy)
    (:`Is Valid`
      (`CancellableAsyncAction.Cancel` (stale `EnhancedInput|/Game/Assets/Input/Actions/IA_Slide` _asynctaskproxy))
      (set `self.IsSliding` false))))

(event `EnhancedInput|/Game/Assets/Input/Actions/IA_Slide`
  (params (ActionValue :type Boolean) (ElapsedSeconds :type "Float (double-precision)") (TriggeredSeconds :type "Float (double-precision)") (InputAction :type "InputAction Object Reference" :default "/Game/Assets/Input/Actions/IA_Slide.IA_Slide"))
  (:`Started`
    (if (not (`self.IsSliding`))
      (set `self.IsSliding` true)
      (`GameplayStatics.PlaySound2D` "/Game/Assets/Sounds/Slide_Player_Cue.Slide_Player_Cue" 1.0 1.0 0.0 null null)
      (bind _asynctaskproxy (`AsyncRootMovement.AsyncRootMovement` (`self.CharacterMovement`) (`self.GetActorForwardVector`) (`self.SlideStrength`) (`self.SlideDuration`) false null "MaintainLastRootMotionVelocity" (0.0 0.0 0.0) 0.0 true)
        (:`OnComplete`
          _)
        (:`OnFail`
          _))
      (set `self.IsSliding` false))))

(event `TriggerInvencibility`
  (bind _capsulecomponent (`self.CapsuleComponent`)
    (:`then`
      (`PrimitiveComponent.SetCollisionResponseToChannel` _capsulecomponent "ECC_Pawn" "ECR_Ignore")
      (bind _returnvalue (`KismetSystemLibrary.K2_SetTimerDelegate` (`|CreateDelegate` :!event `ToggleSpriteFlicker`) (`self.SpriteFlickerTimer`) true))
      (set `self.FlickerHandle` _returnvalue)
      (`KismetSystemLibrary.RetriggerableDelay` (`self.InvencibilityDuration`))
      (`KismetSystemLibrary.K2_ClearAndInvalidateTimerHandle` (`self.FlickerHandle`))
      (`PrimitiveComponent.SetCollisionResponseToChannel` (`self.CapsuleComponent`) "ECC_Pawn" "ECR_Overlap")
      (`SceneComponent.SetVisibility` (`self.Sprite`) true false))
    (:`else`)))

(event `self.ReceiveAnyDamage`
  (params (Damage :type "Float (single-precision)") (DamageType :type "DamageType Object Reference") (InstigatedBy :type "Controller Object Reference") (DamageCauser :type "Actor Object Reference"))
  (bind _returnvalue_x (`KismetMathLibrary.BreakVector` (`KismetMathLibrary.GetForwardVector` (`KismetMathLibrary.FindLookAtRotation` (`self.K2_GetActorLocation`) (`self.K2_GetActorLocation` DamageCauser)))))
  (`parent.ReceiveAnyDamage` Damage DamageType InstigatedBy DamageCauser)
  (`/Game/Widgets/WBP_HealthComponent.UpdateHealth` (`/Game/Widgets/WBP_HUD.WBP_HealthComponent` (`/Game/Blueprints/GM_Action.HUD_Ref` (`self.GameMode`))) (`/Game/Blueprints/Components/BPC_Vitality.CurrentHealth` (`self.BPC_Vitality`)))
  (`self.CancelSlide`)
  (`ActorComponent.Deactivate` (`self.ChargeShot`))
  (set `self.WasHitDuringCharge` true)
  (if (not (`/Game/Blueprints/Components/BPC_Vitality.IsDefeated` (`self.BPC_Vitality`)))
    (`self.TriggerInvencibility`)
    (`GameplayStatics.PlaySound2D` "/Game/Assets/Sounds/Player_Hit_Cue.Player_Hit_Cue" 1.0 1.0 0.0 null null)
    (else
      (`GameplayStatics.PlaySound2D` "/Game/Assets/Sounds/Player_Defeat.Player_Defeat" 1.0 1.0 0.0 null null)))
  (set `CharacterMovementComponent.FallingLateralFriction` 0.0 (`self.CharacterMovement`))
  (`self.LaunchCharacter` (`KismetMathLibrary.MakeVector` (* (`KismetMathLibrary.SelectFloat` -1.0 1.0 (> _returnvalue_x 0.0)) (`self.KnockbackPowerHor`)) 0.0 (`self.KnockbackPowerVer`)) true true)
  (`PaperZDAnimInstance.JumpToNode` (`PaperZDAnimationComponent.AnimInstance` (`self.AnimationComponent`)) "JumpStun" "None")
  (set `self.IsStunned` true)
  (`|ExecutionSequence`
    (:`then_0`
      (`KismetSystemLibrary.RetriggerableDelay` (`self.InvencibilityDuration`))
      (set `CharacterMovementComponent.FallingLateralFriction` (`self.BaseLateralFriction`) (`self.CharacterMovement`)))
    (:`then_1`
      (`KismetSystemLibrary.RetriggerableDelay` (`self.StunDuration`))
      (set `self.IsStunned` false))))

(event `TriggerShootAnim`
  (set `self.IsShooting` true)
  (`KismetSystemLibrary.RetriggerableDelay` (`self.ShootAnimDelay`))
  (set `self.IsShooting` false))

(event `self.OnWalkingOffLedge`
  (params (PreviousFloorImpactNormal :type "Vector Structure (by ref)") (PreviousFloorContactNormal :type "Vector Structure (by ref)") (PreviousLocation :type "Vector Structure (by ref)") (TimeDelta :type "Float (single-precision)"))
  (`self.CancelSlide`))

(event `self.OnLanded`
  (params (Hit :type "HitResult Structure (by ref)"))
  (`GameplayStatics.PlaySound2D` "/Game/Assets/Sounds/Land_Player_Cue.Land_Player_Cue" 1.0 1.0 0.0 null null))

(fn `FlipPlayer`
  (params (Direction :type "Float (double-precision)"))
  (`Controller.SetControlRotation` (`self.GetController`) (select `bool` (>= Direction 0.0) :`false` (`KismetMathLibrary.MakeRotator` 0.0 0.0 180.0) :`true` (`KismetMathLibrary.MakeRotator` 0.0))))

(fn `HandleChargeFlash`
  (params (Elapsed :type "Float (double-precision)"))
  (if (and (not (`self.WasHitDuringCharge`)) (>= Elapsed (`self.PartialChargeTime`)))
    (`ActorComponent.Activate` (`self.ChargeShot`) false)
    (set `self.ChargeFlashTimer` (+ (`self.ChargeFlashTimer`) (`GameplayStatics.GetWorldDeltaSeconds`)))
    (if (>= (`self.ChargeFlashTimer`) (`self.ChargeFlashInterval`))
      (set `self.ChargeFlashTimer` 0.0)
      (`self.TriggerFlash` 5.0 (select `bool` (>= (`local.Elapsed`) (`self.FullChargeTime`)) :`false` (struct :`R` 1.0 :`G` 1.0 :`B` 1.0 :`A` 1.0) :`true` (struct :`R` 0.022275 :`G` 0.16805 :`B` 1.0 :`A` 1.0) :!type "LinearColor Structure")))
    (else
      (set `self.ChargeFlashTimer` 0.0))))

(fn `RestoreShotEnergy`
  (params (ProjectileClass :type "/Game/Blueprints/Projectiles/Player/BP_PlayerProjectile_BASE Class Reference (by ref)"))
  (set `self.ShotEnergy` (`KismetMathLibrary.Min` (+ (`self.ShotEnergy`) (`BlueprintMapLibrary.Map_Find` (`self.ProjectileToEnergy`) (`local.ProjectileClass`))) (`self.ShotEnergyMax`))))

(fn `SpawnProjectile`
  (params (ProjectileClass :type "/Game/Blueprints/Projectiles/Player/BP_PlayerProjectile_BASE Class Reference"))
  (bind (_returnvalue_location _returnvalue_rotation) (`KismetMathLibrary.BreakTransform` (`SceneComponent.K2_GetComponentToWorld` (select `bool` (`self.IsWallSliding`) :`false` (`self.ShootPos`) :`true` (`self.ShootPosWallSlide`)))))
  (if (>= (`self.ShotEnergy`) (`BlueprintMapLibrary.Map_Find` (`self.ProjectileToEnergy`) (`local.ProjectileClass`)))
    (set `self.ShotEnergy` (`KismetMathLibrary.Max` (- (`self.ShotEnergy`) (`BlueprintMapLibrary.Map_Find` (`self.ProjectileToEnergy`) (`local.ProjectileClass`)))))
    (`|SpawnActorFromClass` (`local.ProjectileClass`) (`KismetMathLibrary.MakeTransform` _returnvalue_location _returnvalue_rotation) "AlwaysSpawn" "MultiplyWithRoot" self self)
    (`self.TriggerShootAnim`)
    (`GameplayStatics.PlaySound2D` (select `bool` (== (`local.ProjectileClass`) "/Game/Blueprints/Projectiles/Player/BP_PlayerProjectile_FullCharge.BP_PlayerProjectile_FullCharge_C") :`false` "/Game/Assets/Sounds/Shot_Regular_Cue.Shot_Regular_Cue" :`true` "/Game/Assets/Sounds/Shot_Charged_Cue.Shot_Charged_Cue" :!type "SoundBase Object Reference") 1.0 1.0 0.0 null null)))

(fn `ToggleSpriteFlicker`
  (`SceneComponent.SetVisibility` (`self.Sprite`) (not (`SceneComponent.bVisible` (`self.Sprite`))) false))

(fn `TryChargeShot`
  (params (ElapsedTime :type "Float (double-precision)"))
  (if (not (`self.WasHitDuringCharge`))
    (if (>= ElapsedTime (`self.PartialChargeTime`))
      (if (>= (`local.ElapsedTime`) (`self.FullChargeTime`))
        (`self.SpawnProjectile` "/Game/Blueprints/Projectiles/Player/BP_PlayerProjectile_FullCharge.BP_PlayerProjectile_FullCharge_C")
        (else
          (`self.SpawnProjectile` "/Game/Blueprints/Projectiles/Player/BP_PlayerProjectile_PartialCharge.BP_PlayerProjectile_PartialCharge_C"))))))

(fn `TryWallSlide`
  (bind _returnvalue (`self.K2_GetActorLocation`))
  (bind _returnvalue_x (`KismetMathLibrary.BreakVector` (`self.GetActorForwardVector`)))
  (bind (_velocity_x _velocity_y _velocity_z) (`KismetMathLibrary.BreakVector` (`MovementComponent.Velocity` (`self.CharacterMovement`))))
  (bind (_velocity_x_2 _velocity_y_2 _velocity_z_2) (`KismetMathLibrary.BreakVector` (`MovementComponent.Velocity` (`self.CharacterMovement`))))
  (if (and (<= _velocity_z -50.0) (> (* _returnvalue_x (`|GetInputActionValue`)) 0.0))
    (bind (_outhit _returnvalue_2) (`KismetSystemLibrary.LineTraceSingleForObjects` :`Start` _returnvalue :`End` (+ _returnvalue (* (`self.GetActorForwardVector`) (`self.WallTraceLength`))) :`ObjectTypes` (`|MakeArray` "ObjectTypeQuery1" :!type "EObjectTypeQuery Enum") :`DrawDebugType` "ForOneFrame"))
    (if _returnvalue_2
      (set `self.IsWallSliding` true)
      (set `MovementComponent.Velocity` (`KismetMathLibrary.MakeVector` _velocity_x_2 _velocity_y_2 (`KismetMathLibrary.FMax` _velocity_z_2 (`self.WallSlideSpeed`))) (`self.CharacterMovement`))
      (else
        (set `self.IsWallSliding` false)))
    (else
      (set `self.IsWallSliding` false))))

(fn `UserConstructionScript`
  (`parent.UserConstructionScript`))
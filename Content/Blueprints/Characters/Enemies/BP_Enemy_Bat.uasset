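; Bat enemy that patrols endlessly back and forth between two points, labeled top and bottom.
; On BeginPlay it caches both marker components' world positions, so they stay fixed as the actor moves, then starts a timeline at a configurable play rate.
; The timeline lerps the actor's location without sweeping, and a FlipFlop on completion alternates between reverse and forward playback.
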(event `self.ReceiveBeginPlay`
  (`parent.ReceiveBeginPlay`)
  (set `self.TopPosWorld` (`SceneComponent.K2_GetComponentLocation` (`self.TopPos`)))
  (set `self.BottonPosWorld` (`SceneComponent.K2_GetComponentLocation` (`self.BottonPos`)))
  (`TimelineComponent.SetPlayRate` (`self.MoveAnim`) (`self.MovePlayRate`))
  (`self.MoveForward`))

(event `MoveForward`
  (bind (_direction _alpha) (`Timeline|MoveAnim` :!via `PlayFromStart` :!label _label)
    (:`Update`
      (`self.K2_SetActorLocation` (`KismetMathLibrary.VLerp` (`self.TopPosWorld`) (`self.BottonPosWorld`) _alpha)))
    (:`Finished`
      (`/Engine/EditorBlueprintResources/StandardMacros.FlipFlop`
        (:`A`
          (`self.MoveBackwards`))
        (:`B`
          (`self.MoveForward`))))))

(event `MoveBackwards`
  (goto _label :!via `ReverseFromEnd`))

(fn `UserConstructionScript`
  (`parent.UserConstructionScript`))
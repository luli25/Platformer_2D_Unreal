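; Base projectile actor that damages action characters of an opposing faction on contact.
; Sphere overlap casts to BP_ActionChar_BASE, applies ProjectileDamage only if the Faction differs, then plays the hit effect and destroys itself.
; A blocking sphere hit destroys it with the same effect but no damage.
; PlayHitEffect spawns a BP_VFX_ShotHit actor and plays an impact sound at the projectile's location.
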(event `self.Sphere.OnComponentHit`
  (params (HitComponent :type "PrimitiveComponent Object Reference") (OtherActor :type "Actor Object Reference") (OtherComp :type "PrimitiveComponent Object Reference") (NormalImpulse :type "Vector Structure") (Hit :type "HitResult Structure (by ref)"))
  (`self.PlayHitEffect`)
  (`self.K2_DestroyActor`))

(event `self.Sphere.OnComponentBeginOverlap`
  (params (OverlappedComponent :type "PrimitiveComponent Object Reference") (OtherActor :type "Actor Object Reference") (OtherComp :type "PrimitiveComponent Object Reference") (OtherBodyIndex :type Integer) (bFromSweep :type Boolean) (SweepResult :type "HitResult Structure (by ref)"))
  (bind _asbp_action_char_base (cast `/Game/Blueprints/Characters/BP_ActionChar_BASE` OtherActor))
  (if (`|EnumInequality` (`/Game/Blueprints/Characters/BP_ActionChar_BASE.Faction` _asbp_action_char_base) (`self.Faction`))
    (`GameplayStatics.ApplyDamage` _asbp_action_char_base (`self.ProjectileDamage`) null self)
    (`self.PlayHitEffect`)
    (`self.K2_DestroyActor`)))

(fn `PlayHitEffect`
  (`|SpawnActorFromClass` "/Game/Blueprints/VFX/BP_VFX_ShotHit.BP_VFX_ShotHit_C" (`KismetMathLibrary.MakeTransform` (`self.K2_GetActorLocation`) (`self.K2_GetActorRotation`)) "AlwaysSpawn" "MultiplyWithRoot" null null)
  (`GameplayStatics.PlaySoundAtLocation` "/Game/Assets/Sounds/Destroyed_Projectile_Cue.Destroyed_Projectile_Cue" (`self.K2_GetActorLocation`) (struct) 1.0 1.0 0.0 null null null null))

(fn `UserConstructionScript`)